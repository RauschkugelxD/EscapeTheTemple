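; Menu actor that hosts a menu widget in the world and handles camera transitions to other linked menus.
; On BeginPlay it binds to the widget's transition event, then maps the requested menu type to its linked Main, Credits, Key Bindings, Story or Assets actor.
; A transition swaps collision from this actor to the target and smoothly blends the player's view target to it.
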(event Custom|TransitionTo
  (params (New%20Menu :type Menu%20BP%20Object%20Reference))
  (Collision|SetActorEnableCollision false)
  (Collision|SetActorEnableCollision New%20Menu true)
  (Game|Player|SetViewTargetwithBlend (Game|GetPlayerController 0) New%20Menu 1.0 "VTBlend_EaseInOut" 2.0 false))

(event Custom|OnTrasitionToMenu
  (params (MenuType :type MenuType%20Enum :default "NewEnumerator0"))
  (switch Utilities|FlowControl|Switch|SwitchonMenuType MenuType
    (:NewEnumerator0
      (CallFunction|Transitionto (Variables|Default|GetLinkedMainMenu)))
    (:NewEnumerator1
      (CallFunction|Transitionto (Variables|Default|GetLinkedCreditsMenu)))
    (:NewEnumerator2
      (CallFunction|Transitionto (Variables|Default|GetLinkedKeyBindingsMenu)))
    (:NewEnumerator3
      (CallFunction|Transitionto (Variables|Default|GetLinkedStoryMenu)))
    (:NewEnumerator4
      (CallFunction|Transitionto (Variables|Default|GetLinkedAssetsMenu)))))

(event EventBeginPlay
  (bind _asmenu_base_widget (Utilities|Casting|CastToMenuBaseWidget (UserInterface|GetUserWidgetObject (Variables|Default|GetWidget))))
  (EventDispatchers|BindEventtoTransitiontoLinkedMenu _asmenu_base_widget (delegate Custom|OnTrasitionToMenu)))

(fn ConstructionScript)