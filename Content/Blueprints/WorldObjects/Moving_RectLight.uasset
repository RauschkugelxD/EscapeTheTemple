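; Moving rect light world object that, as wired, plays a breeze sound when the first-person character enters its trigger box.
; The box overlap casts to Custom_FirstPersonCharacter, waits briefly, then plays the 2D sound.
; A ChangeVolume event stores a volume and applies it, clamped, as a sound mix class override.
; The MoveDown timeline that would lower the actor, the player spotlight switch-off and the base mix setup are disconnected.
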(event OnComponentBeginOverlap(Box)
  (params (OverlappedComponent :type Primitive%20Component%20Object%20Reference) (OtherActor :type Actor%20Object%20Reference) (OtherComp :type Primitive%20Component%20Object%20Reference) (OtherBodyIndex :type Integer) (bFromSweep :type Boolean) (SweepResult :type Hit%20Result%20Structure%20%28by%20ref%29))
  (bind _ascustom_first_person_character (Utilities|Casting|CastToCustom_FirstPersonCharacter OtherActor))
  (Utilities|FlowControl|Delay 0.5)
  (Audio|PlaySound2D "/Game/SFX/SoundFiles/Wind/Breeze.Breeze" 1.0 1.0 0.0 0 0))

(event Custom|ChangeVolume
  (params (AudioVolume :type Float%20%28single-precision%29))
  (Variables|Default|SetAudio%20Volume AudioVolume)
  (Audio|SetSoundMixClassOverride 0 0 (Math|Float|Clamp(Float) (Variables|Default|GetAudio%20Volume) 0.01) 1.0 1.0 true))

(fn ConstructionScript)