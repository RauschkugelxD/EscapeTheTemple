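; Fence gate that slides its two halves apart, once, when something overlaps its box.
; The Move timeline lerps each half from its current location toward an offset recomputed every update, sets IsOpen, and plays a delayed gate sound.
; A separate one-shot interaction checks the tool type, then plays the HitGate timeline and sound, but moves nothing because its rotation nodes are disconnected.
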(event OnComponentBeginOverlap(OverlapBox)
  (params (OverlappedComponent :type Primitive%20Component%20Object%20Reference) (OtherActor :type Actor%20Object%20Reference) (OtherComp :type Primitive%20Component%20Object%20Reference) (OtherBodyIndex :type Integer) (bFromSweep :type Boolean) (SweepResult :type Hit%20Result%20Structure%20%28by%20ref%29))
  (bind _fence_left1 (Variables|Default|GetFence_Left1))
  (bind _fence_right1 (Variables|Default|GetFence_Right1))
  (bind _fence_right1_2 (Variables|Default|GetFence_Right1))
  (bind _fence_left1_2 (Variables|Default|GetFence_Left1))
  (bind _relativelocation (Variables|/Script/Engine.SceneComponent|GetRelativeLocation _fence_left1_2))
  (bind _relativelocation_2 (Variables|/Script/Engine.SceneComponent|GetRelativeLocation _fence_left1))
  (bind _relativelocation_3 (Variables|/Script/Engine.SceneComponent|GetRelativeLocation _fence_right1_2))
  ;[1 1 1] Open door
  (Utilities|FlowControl|DoOnce false
    (:Completed
      (Utilities|FlowControl|Sequence
        (:then_0
          (bind _move (Timeline|Move PlayFromStart)
            (:Update
              ;;[1 1 1] Movement Left Door
              (Transformation|SetRelativeLocation _fence_left1 (Math|Vector|Lerp(Vector) _relativelocation_2 (Math|Vector|MakeVector (+ (Variables|Default|GetMove_Distance_Left) (.x _relativelocation)) (.y _relativelocation) (.z _relativelocation)) _move) false false) ; Actual Movement
              ;;[1 1 1] Movement Right Door
              (Transformation|SetRelativeLocation _fence_right1 (Math|Vector|Lerp(Vector) (Variables|/Script/Engine.SceneComponent|GetRelativeLocation _fence_right1) (Math|Vector|MakeVector (+ (Variables|Default|GetMove_Distance_Right) (.x _relativelocation_3)) (.y _relativelocation_3) (.z _relativelocation_3)) _move) false false) ; Actual Movement
              (Variables|Default|SetIsOpen true))))
        (:then_1
          (Utilities|FlowControl|Delay 0.2)
          (Audio|PlaySoundatLocation "/Game/SFX/MetalGate_short.MetalGate_short" _relativelocation_2 "0, 0, 0" 1.0 1.0 0.0 0 0 0) ; SFX
        )))))

(event EventBeginInteraction
  (params (Interactor :type ToolType%20Enum :default "NewEnumerator1"))
  ;[1 1 1] Check if player hasn't interacted yet and interacts with specific object
  (if (not (Variables|Default|GetHasInteracted))
    (bind _can_interact (CallFunction|CheckToolType Interactor))
    (if _can_interact
      (Utilities|FlowControl|DoOnce false
        (:Completed
          (Utilities|FlowControl|Sequence
            (:then_0
              (bind _hit (Timeline|HitGate PlayFromStart)
                (:Update
                  (if true
                    _))))
            (:then_1
              (Utilities|FlowControl|Delay 0.2)
              (Audio|PlaySoundatLocation "/Game/SFX/MetalGate_short.MetalGate_short" "0, 0, 0" "0, 0, 0" 1.0 1.0 0.0 0 0 0) ; SFX
            )))))))

(fn ConstructionScript)

(fn CheckToolType
  (params (Tool%20Type :type ToolType%20Enum :default "NewEnumerator1"))
  (if (Variables|Default|GetHasInteracted)
    (return false)
    (else
      (return (Utilities|Enum|Equal(Enum) Tool%20Type "NewEnumerator5")))))