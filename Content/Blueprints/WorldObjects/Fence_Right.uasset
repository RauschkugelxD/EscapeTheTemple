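; Right-hand fence world object that slides along relative X on box overlap and rotates when hit with a specific tool.
; The overlap fires once, driving the Move timeline and a delayed metal gate sound.
; CheckToolType accepts two hits, each playing its own timeline toward a different rotation, with sound only on the first.
; All three timelines lerp from the fence's current transform each update rather than a cached start.
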(event OnComponentBeginOverlap(OverlapBox)
  (params (OverlappedComponent :type Primitive%20Component%20Object%20Reference) (OtherActor :type Actor%20Object%20Reference) (OtherComp :type Primitive%20Component%20Object%20Reference) (OtherBodyIndex :type Integer) (bFromSweep :type Boolean) (SweepResult :type Hit%20Result%20Structure%20%28by%20ref%29))
  (bind _fence_right1 (Variables|Default|GetFence_Right1))
  (bind _fence_right1_2 (Variables|Default|GetFence_Right1))
  (bind _relativelocation (Variables|/Script/Engine.SceneComponent|GetRelativeLocation _fence_right1_2))
  ;[1 1 1] Slide fence from right to left
  (Utilities|FlowControl|DoOnce false
    (:Completed
      (Utilities|FlowControl|Sequence
        (:then_0
          (bind _move (Timeline|Move PlayFromStart)
            (:Update
              ;;[1 1 1] Movement Right Door
              (Transformation|SetRelativeLocation _fence_right1 (Math|Vector|Lerp(Vector) (Variables|/Script/Engine.SceneComponent|GetRelativeLocation _fence_right1) (Math|Vector|MakeVector (+ (Variables|Default|GetMove_Distance_Right) (.x _relativelocation)) (.y _relativelocation) (.z _relativelocation)) _move) false false) ; Actual Movement
            )))
        (:then_1
          (Utilities|FlowControl|Delay 0.2)
          (Audio|PlaySoundatLocation "/Game/SFX/MetalGate_short.MetalGate_short" "0, 0, 0" "0, 0, 0" 1.0 1.0 0.0 0 0 0) ; SFX
        )))))

(event EventBeginInteraction
  (params (Interactor :type ToolType%20Enum :default "NewEnumerator1"))
  ;[1 1 1] Check if player hasn't interacted yet and interacts with specific object
  (bind _can_interact (CallFunction|CheckToolType Interactor))
  (if _can_interact
    (Math|Integer|IncrementInt (Variables|Default|GetHitCounter)
      (:%20%20
        (if (== (Variables|Default|GetHitCounter) 1)
          (Utilities|FlowControl|Sequence
            (:then_0
              ;[1 1 1] Rotation
              (bind _hit (Timeline|HitGate Play)
                (:Update
                  (Transformation|SetRelativeRotation (Variables|Default|GetFence_Right1) (Math|Rotator|Lerp(Rotator) (Variables|/Script/Engine.SceneComponent|GetRelativeRotation (Variables|Default|GetFence_Right1)) (Variables|Default|GetRotate_End1) _hit) false false))))
            (:then_1
              ;[1 1 1] SFX
              (Utilities|FlowControl|Delay 0.2)
              (Audio|PlaySoundatLocation "/Game/SFX/MetalGate_short.MetalGate_short" "0, 0, 0" "0, 0, 0" 1.0 1.0 0.0 0 0 0) ; SFX
            ))
          (else
            (Utilities|FlowControl|Sequence
              (:then_0
                ;[1 1 1] Rotation
                (bind _hit_2 (Timeline|Timeline_0 Play)
                  (:Update
                    (Transformation|SetRelativeRotation (Variables|Default|GetFence_Right1) (Math|Rotator|Lerp(Rotator) (Variables|/Script/Engine.SceneComponent|GetRelativeRotation (Variables|Default|GetFence_Right1)) (Variables|Default|GetEndPoint2) _hit_2) false false))))
              (:then_1
                ;[1 1 1] SFX
                (Utilities|FlowControl|Delay 0.2)))))))))

(fn ConstructionScript)

(fn CheckToolType
  (params (Tool%20Type :type ToolType%20Enum :default "NewEnumerator1"))
  (if (< (Variables|Default|GetHitCounter) 2)
    (if (Utilities|Enum|Equal(Enum) Tool%20Type "NewEnumerator5")
      (return true)
      (else
        (return false)))
    (else
      (return false))))