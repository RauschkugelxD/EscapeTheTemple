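; Base item actor that carries an ItemStructure and exposes it, along with the item's name, through getters.
; CheckToolType always returns false here.
; BeginInteraction is empty, with a TODO questioning whether it is still needed.
; Disconnected pickup logic would add one item to an actor's InventoryComponent and destroy this actor on success, but never runs.
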(event EventBeginInteraction
  (params (Interactor :type ToolType%20Enum :default "NewEnumerator1"))
  ;[1 1 1] TODO: Is this part still needed? (@ Lisa)
)

(fn ConstructionScript)

(fn GetItemName
  (return (.Name (Utilities|Struct|BreakItemStructure (Variables|Default|GetItemStructure)))))

(fn GetItemStructure
  (return (Variables|Default|GetItemStructure)))

(fn CheckToolType
  (params (Tool%20Type :type ToolType%20Enum :default "NewEnumerator1"))
  (return false))