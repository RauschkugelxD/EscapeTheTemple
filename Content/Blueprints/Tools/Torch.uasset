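; Torch tool that can be lit once by interacting with a specific tool type, showing its fire component and disabling the mesh's shadow casting.
; IsLit drives the construction-time fire visibility, blocks further interaction once lit, and switches the tool type the torch reports.
; State get and set functions expose IsLit, with a true state reusing the lighting path and a false state doing nothing.
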(event EventSetCurrentState
  (params (State :type Object%20Object%20Reference) (BoolState :type Boolean))
  (if BoolState
    ;[1 1 1] Light up the torch
    (Rendering|SetVisibility (Variables|Default|GetFire_BP) true false)
    (bind _output_get (Variables|Default|SetIsLit true))
    ;;[1 1 1] Don't cast shadows on itself
    (Rendering|SetCastShadow (Variables|Default|GetStaticMesh) (not _output_get))))

(event EventBeginInteraction
  (params (Interactor :type ToolType%20Enum :default "NewEnumerator1"))
  ;[1 1 1] Light up the torch
  (if (Utilities|Enum|Equal(Enum) Interactor "NewEnumerator4")
    (Rendering|SetVisibility (Variables|Default|GetFire_BP) true false)
    (bind _output_get (Variables|Default|SetIsLit true))
    ;;[1 1 1] Don't cast shadows on itself
    (Rendering|SetCastShadow (Variables|Default|GetStaticMesh) (not _output_get))))

(fn ConstructionScript
  (Rendering|SetVisibility (Variables|Default|GetFire_BP) (Variables|Default|GetIsLit) false))

(fn CheckToolType
  (params (Tool%20Type :type ToolType%20Enum :default "NewEnumerator1"))
  (if (not (Variables|Default|GetIsLit)) ; If torch is already lit up, no interaction possible
    (return (Utilities|Enum|Equal(Enum) Tool%20Type "NewEnumerator4"))))

(fn GetItemStructure
  (return (Variables|Default|GetItem_Structure)))

(fn GetCurrentState
  (return 0 (Variables|Default|GetIsLit)))

(fn GetToolType
  (if (Variables|Default|GetIsLit)
    (return "NewEnumerator8")
    (else
      (return "NewEnumerator1"))))