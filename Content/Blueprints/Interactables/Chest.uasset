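; Interactable chest that opens once when the player interacts with it by hand.
; BeginInteraction runs a tool-type enum check, then a DoOnce gate starts two delayed branches.
; One plays the Rotate timeline, lerping the lid from its current rotation toward the open angle and setting IsOpen.
; The other plays the opening sound at the lid's location, ahead of the rotation.
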(event EventBeginInteraction
  (params (Interactor :type ToolType%20Enum :default "NewEnumerator1"))
  (bind _chest_lid (Variables|Default|GetChest_Lid))
  ;[1 1 1] Open chest
  ;;[1 1 1] Check if player interacts with hand
  (bind _can_interact (CallFunction|CheckToolType Interactor))
  (if _can_interact
    (Utilities|FlowControl|DoOnce false
      (:Completed
        (Utilities|FlowControl|Sequence
          (:then_0
            (Utilities|FlowControl|Delay 0.6)
            ;;[1 1 1] Rotation
            (bind _hit (Timeline|Rotate PlayFromStart)
              (:Update
                (Transformation|SetRelativeRotation _chest_lid (Math|Rotator|Lerp(Rotator) (Variables|/Script/Engine.SceneComponent|GetRelativeRotation _chest_lid) "0,0.000000,110.000000" _hit) false false)
                (Variables|Default|SetIsOpen true))))
          (:then_1
            ;;[1 1 1] SFX
            (Utilities|FlowControl|Delay 0.1)
            (Audio|PlaySoundatLocation "/Game/SFX/SoundFiles/Chest_opening.Chest_opening" (Transformation|GetWorldLocation _chest_lid) "0, 0, 0" 1.0 1.0 0.0 0 0 0) ; SFX
          ))))))

(fn ConstructionScript)

(fn CheckToolType
  (params (Tool%20Type :type ToolType%20Enum :default "NewEnumerator1"))
  (if (Utilities|Enum|Equal(Enum) Tool%20Type "NewEnumerator7")
    (return true)
    (else
      (return false))))