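; An interactable elevator that raises its static mesh along Z when a matching tool type interacts with it.
; BeginInteraction passes the interactor to CheckToolType, which accepts one specific enum value, then plays a timeline.
; Each timeline update lerps relative location from the mesh's current position toward that position plus MoveDistance, using the Move curve as alpha, so offsets accumulate rather than interpolating between fixed endpoints.
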(event EventBeginInteraction
  (params (Interactor :type ToolType%20Enum :default "NewEnumerator1"))
  (bind _staticmesh (Variables|Default|GetStaticMesh))
  (bind _staticmesh_2 (Variables|Default|GetStaticMesh))
  (bind _relativelocation (Variables|/Script/Engine.SceneComponent|GetRelativeLocation _staticmesh_2))
  (bind _can_interact (CallFunction|CheckToolType Interactor))
  (if _can_interact
    ;[1 1 1] Movement according to curve of timeline
    (bind _move (Timeline|Timeline_0 Play)
      (:Update
        (Transformation|SetRelativeLocation _staticmesh (Math|Vector|Lerp(Vector) (Variables|/Script/Engine.SceneComponent|GetRelativeLocation _staticmesh) (Math|Vector|MakeVector (.x _relativelocation) (.y _relativelocation) (+ (Variables|Components|GetMoveDistance) (.z _relativelocation))) _move) false false) ; Actual Movement
      ))))

(fn ConstructionScript)

(fn CheckToolType
  (params (Tool%20Type :type ToolType%20Enum :default "NewEnumerator1"))
  (return (Utilities|Enum|Equal(Enum) Tool%20Type "NewEnumerator7")))