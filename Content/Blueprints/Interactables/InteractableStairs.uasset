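; Interactable stairs that move vertically when their child-actor StairsSwitch is switched.
; The construction script binds the switch's OnSwitched event and passes it the linked braziers.
; On switching, the stairs disable further switch interaction, play a door sound after a short delay and run a timeline.
; Each timeline update lerps the mesh from its current relative location toward a Z offset of MoveDistance, so movement accumulates.
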(event Custom|On%20Stairs%20Switched
  (bind _stairs_mesh (Variables|Default|GetStairs%20mesh))
  (bind _stairs_mesh_2 (Variables|Default|GetStairs%20mesh))
  (bind _relativelocation (Variables|/Script/Engine.SceneComponent|GetRelativeLocation _stairs_mesh))
  (bind _relativelocation_2 (Variables|/Script/Engine.SceneComponent|GetRelativeLocation _stairs_mesh_2))
  (bind _asstairs_switch (Utilities|Casting|CastToStairsSwitch (Variables|/Script/Engine.ChildActorComponent|GetChildActor (Variables|Default|GetStairsSwitch))))
  (Variables|/Game/Blueprints/Interactables/StairsSwitch.StairsSwitch_C|SetShallInteract _asstairs_switch false)
  (Utilities|FlowControl|Sequence
    (:then_0
      ;[1 1 1] Movement according to curve of timeline
      (bind _move (Timeline|Timeline_0 PlayFromStart)
        (:Update
          (Transformation|SetRelativeLocation _stairs_mesh_2 (Math|Vector|Lerp(Vector) _relativelocation_2 (Math|Vector|MakeVector (.x _relativelocation) (.y _relativelocation) (+ (Variables|Default|GetMoveDistance) (.z _relativelocation))) _move) false false) ; Actual Movement
        )))
    (:then_1
      (Utilities|FlowControl|Delay 0.2)
      (Audio|PlaySoundatLocation "/Game/SFX/SoundFiles/Rocks/MovingDoor_2.MovingDoor_2" _relativelocation_2 "0, 0, 0" 1.0 1.0 0.0 0 0 0) ; SFX
    )))

(fn ConstructionScript
  (bind _asstairs_switch (Utilities|Casting|CastToStairsSwitch (Variables|/Script/Engine.ChildActorComponent|GetChildActor (Variables|Default|GetStairsSwitch))))
  (EventDispatchers|BindEventtoOnSwitched _asstairs_switch (EventDispatchers|CreateEvent :!event Custom|On%20Stairs%20Switched))
  (Variables|/Game/Blueprints/Interactables/StairsSwitch.StairsSwitch_C|SetLinkedBraziers _asstairs_switch (Variables|Default|GetLinkedBraziers)))