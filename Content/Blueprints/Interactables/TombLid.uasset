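; Interactable tomb lid that slides aside once when used with one specific tool type, then drops.
; A timeline curve drives a lerp on the mesh's relative Y, each update offsetting from its current position by MoveDistance, then physics is enabled when it finishes.
; Delayed slide and impact sounds play in parallel.
; CheckToolType reports whether a tool is valid, returning false once the lid has been moved.
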(event EventBeginInteraction
  (params (Interactor :type ToolType%20Enum :default "NewEnumerator1"))
  (bind _staticmesh (Variables|Default|GetStaticMesh))
  (bind _staticmesh_2 (Variables|Default|GetStaticMesh))
  (bind _relativelocation (Variables|/Script/Engine.SceneComponent|GetRelativeLocation _staticmesh_2))
  (bind _relativelocation_2 (Variables|/Script/Engine.SceneComponent|GetRelativeLocation _staticmesh))
  ;[1 1 1] Handling of movement of the tomb lid
  ;;[1 1 1] Check the tool the player interacts with
  (if (not (Variables|Default|GetHasInteracted))
    (if (Utilities|Enum|Equal(Enum) Interactor "NewEnumerator2")
      (Utilities|FlowControl|Sequence
        (:then_0
          ;;[1 1 1] Movement according to curve of timeline
          (bind _move (Timeline|Timeline_0 PlayFromStart)
            (:Update
              (Transformation|SetRelativeLocation _staticmesh (Math|Vector|Lerp(Vector) _relativelocation_2 (Math|Vector|MakeVector (.x _relativelocation) (+ (Variables|Default|GetMoveDistance) (.y _relativelocation)) (.z _relativelocation)) _move) false false) ; Actual Movement
              (Variables|Default|SetHasInteracted true))
            (:Finished
              (Physics|SetSimulatePhysics _staticmesh true) ; Let lid fall down
            )))
        (:then_1
          ;;[1 1 1] Play sound effects
          (Utilities|FlowControl|Delay 0.2)
          (Audio|PlaySoundatLocation "/Game/SFX/SoundFiles/Rocks/TombLid_2.TombLid_2" _relativelocation_2 "0, 0, 0" 1.0 1.0 0.0 0 0 0) ; SFX
          (Utilities|FlowControl|Delay 1.4)
          (Audio|PlaySoundatLocation "/Game/SFX/SoundFiles/Rocks/TombLid_Hit_1.TombLid_Hit_1" _relativelocation_2 "0, 0, 0" 1.0 1.0 0.0 0 0 0) ; SFX
        )))))

(fn ConstructionScript)

(fn CheckToolType
  (params (Tool%20Type :type ToolType%20Enum :default "NewEnumerator1"))
  (if (Variables|Default|GetHasInteracted)
    (return false)
    (else
      (return (Utilities|Enum|Equal(Enum) Tool%20Type "NewEnumerator2")))))