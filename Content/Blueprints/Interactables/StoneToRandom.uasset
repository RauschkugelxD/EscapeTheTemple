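; Interactable stone prop that a specific tool type turns, one time only, into a random runic stone figure.
; The Construction Script gives it a random big or mid rock mesh.
; On BeginInteraction, CheckToolType tests the tool enum and the IsStoneFigure flag, then the flag is set and a random runic mesh replaces a briefly assigned Bow mesh.
; The runic roll is weighted toward the seventh mesh, since the higher results all fall through to it.
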(event EventBeginInteraction
  (params (Interactor :type ToolType%20Enum :default "NewEnumerator1"))
  (bind _staticmesh (Variables|Default|GetStaticMesh))
  (bind _can_interact (CallFunction|CheckToolType Interactor))
  (if _can_interact
    (Components|StaticMesh|SetStaticMesh (Variables|Default|GetStaticMesh) "/Game/StaticMeshes/TempleOnHill/Bow.Bow")
    (Variables|Default|SetIsStoneFigure true)
    (switch int (Math|Random|RandomInteger 11)
      (:Default
        (Components|StaticMesh|SetStaticMesh _staticmesh "/Game/StaticMeshes/StonePack/Stonepack_Runic_7.Stonepack_Runic_7" :!label _label))
      (:0
        (Components|StaticMesh|SetStaticMesh _staticmesh "/Game/StaticMeshes/StonePack/Stonepack_Runic_1.Stonepack_Runic_1"))
      (:1
        (Components|StaticMesh|SetStaticMesh _staticmesh "/Game/StaticMeshes/StonePack/Stonepack_Runic_2.Stonepack_Runic_2"))
      (:2
        (Components|StaticMesh|SetStaticMesh _staticmesh "/Game/StaticMeshes/StonePack/Stonepack_Runic_3.Stonepack_Runic_3"))
      (:3
        (Components|StaticMesh|SetStaticMesh _staticmesh "/Game/StaticMeshes/StonePack/Stonepack_Runic_4.Stonepack_Runic_4"))
      (:4
        (Components|StaticMesh|SetStaticMesh _staticmesh "/Game/StaticMeshes/StonePack/Stonepack_Runic_5.Stonepack_Runic_5"))
      (:5
        (Components|StaticMesh|SetStaticMesh _staticmesh "/Game/StaticMeshes/StonePack/Stonepack_Runic_6.Stonepack_Runic_6"))
      (:6
        (goto _label)))))

(fn ConstructionScript
  (bind _staticmesh (Variables|Default|GetStaticMesh))
  (switch int (Math|Random|RandomInteger 11)
    (:Default
      (Components|StaticMesh|SetStaticMesh _staticmesh "/Game/StaticMeshes/StonePack/Stonepack_Mid_41.Stonepack_Mid_41" :!label _label))
    (:0
      (Components|StaticMesh|SetStaticMesh _staticmesh "/Game/StaticMeshes/StonePack/Stonepack_BIG_1.Stonepack_BIG_1"))
    (:1
      (Components|StaticMesh|SetStaticMesh _staticmesh "/Game/StaticMeshes/StonePack/Stonepack_Big_2.Stonepack_Big_2"))
    (:2
      (Components|StaticMesh|SetStaticMesh _staticmesh "/Game/StaticMeshes/StonePack/Stonepack_Big_3.Stonepack_Big_3"))
    (:3
      (Components|StaticMesh|SetStaticMesh _staticmesh "/Game/StaticMeshes/StonePack/Stonepack_Big_4.Stonepack_Big_4"))
    (:4
      (Components|StaticMesh|SetStaticMesh _staticmesh "/Game/StaticMeshes/StonePack/Stonepack_Big_5.Stonepack_Big_5"))
    (:5
      (Components|StaticMesh|SetStaticMesh _staticmesh "/Game/StaticMeshes/StonePack/Stonepack_Mid_1.Stonepack_Mid_1"))
    (:6
      (Components|StaticMesh|SetStaticMesh _staticmesh "/Game/StaticMeshes/StonePack/Stonepack_Mid_2.Stonepack_Mid_2"))
    (:7
      (Components|StaticMesh|SetStaticMesh _staticmesh "/Game/StaticMeshes/StonePack/Stonepack_Mid_3.Stonepack_Mid_3"))
    (:8
      (Components|StaticMesh|SetStaticMesh _staticmesh "/Game/StaticMeshes/StonePack/Stonepack_Mid_4.Stonepack_Mid_4"))
    (:9
      (Components|StaticMesh|SetStaticMesh _staticmesh "/Game/StaticMeshes/StonePack/Stonepack_Mid_5.Stonepack_Mid_5"))
    (:10
      (goto _label))))

(fn CheckToolType
  (params (Tool%20Type :type ToolType%20Enum :default "NewEnumerator1"))
  (return (and (Utilities|Enum|Equal(Enum) Tool%20Type "NewEnumerator11") (not (Variables|Default|GetIsStoneFigure)))))