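; Collectable pickup actor that the first-person player collects by walking into its Box trigger.
; On begin overlap with Custom_FirstPersonCharacter, it decrements CollectablesLeft on FirstPersonGameMode, adds a new Collectable_Widget to the viewport and destroys itself.
; The end-overlap event repeats the character and game mode casts but takes no further action.
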(event OnComponentBeginOverlap(Box)
  (params (OverlappedComponent :type Primitive%20Component%20Object%20Reference) (OtherActor :type Actor%20Object%20Reference) (OtherComp :type Primitive%20Component%20Object%20Reference) (OtherBodyIndex :type Integer) (bFromSweep :type Boolean) (SweepResult :type Hit%20Result%20Structure%20%28by%20ref%29))
  (Utilities|Casting|CastToCustom_FirstPersonCharacter OtherActor) ; Check if correct character is overlapping the box
  ;[1 1 1] Recompute left collectables
  (bind _asfirst_person_game_mode (Utilities|Casting|CastToFirstPersonGameMode (Game|GetGameMode)))
  (bind _result (Math|Integer|DecrementInt (Variables|/Game/Blueprints/GameFunctionality/FirstPersonGameMode.FirstPersonGameMode_C|GetCollectables_Left _asfirst_person_game_mode)) ; Subtract 1
    (:%20%20
      (Variables|/Game/Blueprints/GameFunctionality/FirstPersonGameMode.FirstPersonGameMode_C|SetCollectables_Left _asfirst_person_game_mode _result)
      ;[1 1 1] Show widget
      (bind _returnvalue (UserInterface|CreateWidget "/Game/Blueprints/UserInterface/Collectable_Widget.Collectable_Widget_C"))
      (UserInterface|Viewport|AddtoViewport _returnvalue 0)
      (Actor|DestroyActor))))

(event OnComponentEndOverlap(Box)
  (params (OverlappedComponent :type Primitive%20Component%20Object%20Reference) (OtherActor :type Actor%20Object%20Reference) (OtherComp :type Primitive%20Component%20Object%20Reference) (OtherBodyIndex :type Integer))
  (Utilities|Casting|CastToCustom_FirstPersonCharacter OtherActor) ; Check if correct character is overlapping the box
  (Utilities|Casting|CastToFirstPersonGameMode (Game|GetGameMode)))

(fn ConstructionScript)