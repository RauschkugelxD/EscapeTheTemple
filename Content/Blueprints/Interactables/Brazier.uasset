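; Brazier interactable that the player can light with a suitable tool.
; On interaction it accepts only two specific tool types while unlit, then shows the fire component, sets IsLit and calls the OnLight dispatcher for listeners.
; The construction script hides the fire when IsLit is false, so each instance's starting state shows in the editor.
; No logic here extinguishes it once lit.
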(event EventBeginInteraction
  (params (Interactor :type ToolType%20Enum :default "NewEnumerator1"))
  (bind _can_interact (CallFunction|CheckToolType Interactor))
  (if _can_interact
    (Rendering|SetVisibility (Variables|Default|GetFire_BP) true false)
    (Variables|Default|SetIsLit true)
    (Default|CallOnLight)))

(fn ConstructionScript
  (if (not (Variables|Default|GetIsLit))
    (Rendering|SetVisibility (Variables|Default|GetFire_BP) false false)))

(fn CheckToolType
  (params (Tool%20Type :type ToolType%20Enum :default "NewEnumerator1"))
  (return (and (or (Utilities|Enum|Equal(Enum) Tool%20Type "NewEnumerator8") (Utilities|Enum|Equal(Enum) Tool%20Type "NewEnumerator4")) (not (Variables|Default|GetIsLit)))))