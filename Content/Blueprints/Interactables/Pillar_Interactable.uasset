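; An interactable pillar that the player knocks over once by hitting it with a specific tool type from the correct side.
; An overlap box marks the wrong side, disabling interaction while the player is inside and enabling it once they leave.
; A valid hit runs a one-time timeline that rotates the pillar downwards, with a delayed impact sound.
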(event OnComponentBeginOverlap(OverlapBox)
  (params (OverlappedComponent :type Primitive%20Component%20Object%20Reference) (OtherActor :type Actor%20Object%20Reference) (OtherComp :type Primitive%20Component%20Object%20Reference) (OtherBodyIndex :type Integer) (bFromSweep :type Boolean) (SweepResult :type Hit%20Result%20Structure%20%28by%20ref%29))
  ;[1 1 1] If player enters collision box on wrong side of pillar, interaction is not possible
  (Utilities|Casting|CastToCustom_FirstPersonCharacter OtherActor)
  (Variables|Default|SetIsAtPosition false))

(event OnComponentEndOverlap(OverlapBox)
  (params (OverlappedComponent :type Primitive%20Component%20Object%20Reference) (OtherActor :type Actor%20Object%20Reference) (OtherComp :type Primitive%20Component%20Object%20Reference) (OtherBodyIndex :type Integer))
  ;[1 1 1] If player is on correct side of pillar, interaction is possible
  (Utilities|Casting|CastToCustom_FirstPersonCharacter OtherActor)
  (Variables|Default|SetIsAtPosition true))

(event EventBeginInteraction
  (params (Interactor :type ToolType%20Enum :default "NewEnumerator1"))
  (bind _pillar (Variables|Default|GetPillar))
  ;[1 1 1] Hit pillar
  ;;[1 1 1] Check if player is at correct position with correct tool
  (if (Variables|Default|GetIsAtPosition)
    (bind _can_interact (CallFunction|CheckToolType Interactor))
    (if _can_interact
      (Variables|Default|SetHasInteracted true)
      (Utilities|FlowControl|DoOnce false
        (:Completed
          (Utilities|FlowControl|Sequence
            (:then_0
              ;;[1 1 1] Rotate pillar downwards
              (bind _move (Timeline|Rotate PlayFromStart)
                (:Update
                  (Transformation|SetRelativeRotation _pillar (Math|Rotator|Lerp(Rotator) (Variables|/Script/Engine.SceneComponent|GetRelativeRotation _pillar) "0,0.000000,-90.000000" _move) false false))))
            (:then_1
              ;;[1 1 1] SFX
              (Utilities|FlowControl|Delay 1.1)
              (Audio|PlaySoundatLocation "/Game/SFX/TombLid_Hit_1.TombLid_Hit_1" (Variables|/Script/Engine.SceneComponent|GetRelativeLocation _pillar) "0, 0, 0" 1.0 1.0 0.0 0 0 0) ; SFX
            )))))))

(fn ConstructionScript)

(fn CheckToolType
  (params (Tool%20Type :type ToolType%20Enum :default "NewEnumerator1"))
  (if (Variables|Default|GetHasInteracted)
    (return false)
    (else
      (return (Utilities|Enum|Equal(Enum) Tool%20Type "NewEnumerator2")))))