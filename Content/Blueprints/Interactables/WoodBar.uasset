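; WoodBar is an interactable wooden bar that breaks into three loose pieces.
; On BeginInteraction it destroys the intact StaticMesh component, then reveals the three WoodPart components and enables physics simulation on them.
; CheckToolType reports whether a given tool is one of two accepted enum types, while the interaction event itself performs no tool check.
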(event EventBeginInteraction
  (params (Interactor :type ToolType%20Enum :default "NewEnumerator1"))
  (Components|DestroyComponent (Variables|Default|GetStaticMesh))
  (Rendering|SetVisibility (Variables|Default|GetWoodPart1) true false)
  (Rendering|SetVisibility (Variables|Default|GetWoodPart2) true false)
  (Rendering|SetVisibility (Variables|Default|GetWoodPart3) true false)
  (Physics|SetSimulatePhysics (Variables|Default|GetWoodPart1) true)
  (Physics|SetSimulatePhysics (Variables|Default|GetWoodPart2) true)
  (Physics|SetSimulatePhysics (Variables|Default|GetWoodPart3) true))

(fn ConstructionScript)

(fn CheckToolType
  (params (Tool%20Type :type ToolType%20Enum :default "NewEnumerator1"))
  (return (or (Utilities|Enum|Equal(Enum) Tool%20Type "NewEnumerator10") (Utilities|Enum|Equal(Enum) Tool%20Type "NewEnumerator9"))))