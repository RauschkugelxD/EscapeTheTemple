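; Pressure plate that opens the Crypt2_Gate when an actor begins overlapping its box and closes it when an overlap ends.
; Two timelines move the plate down and up with press and release sounds.
; Two DoOnce nodes gate press and release, each reset by the opposite movement's timeline.
; Checks for remaining occupants, pressed state and gate state are disconnected, so any actor leaving can trigger release.
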(event OnComponentBeginOverlap(OverlapBox)
  (params (OverlappedComponent :type Primitive%20Component%20Object%20Reference) (OtherActor :type Actor%20Object%20Reference) (OtherComp :type Primitive%20Component%20Object%20Reference) (OtherBodyIndex :type Integer) (bFromSweep :type Boolean) (SweepResult :type Hit%20Result%20Structure%20%28by%20ref%29))
  (bind _pressureplate (Variables|Default|GetPressurePlate))
  ;[1 1 1] Move pressure plate
  ;;[1 1 1] Variable check
  (Variables|Default|SetIsPressed true)
  (Utilities|FlowControl|DoOnce false
    (:Completed
      ;;[1 1 1] Move pressure plate downwards
      (Utilities|FlowControl|Sequence
        (:then_0
          (bind _move (Timeline|MoveDown PlayFromStart)
            (:Update
              (Transformation|SetRelativeLocation _pressureplate (Math|Vector|MakeVector 0.0 0.0 _move) false false) ; Actual Movement
              (Utilities|FlowControl|DoOnce false) ; enters at Reset
            )))
        (:then_1
          ;;[1 1 1] SFX
          (Utilities|FlowControl|Delay 0.1)
          (Audio|PlaySoundatLocation "/Game/SFX/SoundFiles/Rocks/Pressure_Plate_1.Pressure_Plate_1" (Variables|/Script/Engine.SceneComponent|GetRelativeLocation _pressureplate) "0, 0, 0" 1.0 1.0 0.0 0 0 0) ; SFX
        )
        (:then_2
          ;;[1 1 1] Open gate
          (bind _returnvalue (Actor|GetActorOfClass "/Game/Blueprints/Interactables/Doors/Crypt2_Gate.Crypt2_Gate_C"))
          (Default|OpenGate _returnvalue))))))

(event OnComponentEndOverlap(OverlapBox)
  (params (OverlappedComponent :type Primitive%20Component%20Object%20Reference) (OtherActor :type Actor%20Object%20Reference) (OtherComp :type Primitive%20Component%20Object%20Reference) (OtherBodyIndex :type Integer))
  (bind _pressureplate (Variables|Default|GetPressurePlate))
  ;[1 1 1] Move pressure plate
  ;;[1 1 1] Variable check
  (Variables|Default|SetIsPressed false)
  (Utilities|FlowControl|DoOnce false
    (:Completed
      ;;[1 1 1] SFX
      (Utilities|FlowControl|Sequence
        (:then_0
          ;;[1 1 1] Move pressure plate upwards
          (bind _move (Timeline|Timeline_0 ReverseFromEnd)
            (:Update
              (Transformation|SetRelativeLocation (Variables|Default|GetPressurePlate) (Math|Vector|MakeVector 0.0 0.0 _move) false false) ; Actual Movement
              (Utilities|FlowControl|DoOnce false) ; enters at Reset
            )))
        (:then_1
          (Audio|PlaySoundatLocation "/Game/SFX/SoundFiles/Rocks/Pressure_Plate_2.Pressure_Plate_2" (Variables|/Script/Engine.SceneComponent|GetRelativeLocation (Variables|Default|GetPressurePlate)) "0, 0, 0" 1.0 1.0 0.0 0 0 0) ; SFX
        )
        (:then_2
          ;[1 1 1] Close gate
          (bind _returnvalue (Actor|GetActorOfClass "/Game/Blueprints/Interactables/Doors/Crypt2_Gate.Crypt2_Gate_C"))
          (Default|CloseGate _returnvalue))))))

(fn ConstructionScript)