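; StoneToStar is an interactable prop that turns one-way from its initial stone state into a star state.
; Interacting with the required tool type while not yet a star swaps the static mesh to a barrel keg mesh and sets IsStar.
; SetCurrentState reapplies that change when passed true, and GetCurrentState reports the flag.
; GetToolType returns a different enum value per state, and GetItemStructure exposes its item data.
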(event EventSetCurrentState
  (params (State :type Object%20Object%20Reference) (BoolState :type Boolean))
  (if BoolState
    (Components|StaticMesh|SetStaticMesh (Variables|Default|GetStaticMesh) "/Game/StaticMeshes/Barrel/Barrel_Low_Keg_low.Barrel_Low_Keg_low")
    (Variables|Default|SetIsStar true)))

(event EventBeginInteraction
  (params (Interactor :type ToolType%20Enum :default "NewEnumerator1"))
  (bind _can_interact (CallFunction|CheckToolType Interactor))
  (if _can_interact
    (Components|StaticMesh|SetStaticMesh (Variables|Default|GetStaticMesh) "/Game/StaticMeshes/Barrel/Barrel_Low_Keg_low.Barrel_Low_Keg_low")
    (Variables|Default|SetIsStar true)))

(fn ConstructionScript)

(fn CheckToolType
  (params (Tool%20Type :type ToolType%20Enum :default "NewEnumerator1"))
  (return (and (Utilities|Enum|Equal(Enum) Tool%20Type "NewEnumerator11") (not (Variables|Default|GetIsStar)))))

(fn GetItemStructure
  (return (Variables|Components|GetItem_Structure)))

(fn GetCurrentState
  (return 0 (Variables|Default|GetIsStar)))

(fn GetToolType
  (if (Variables|Default|GetIsStar)
    (return "NewEnumerator20")
    (else
      (return "NewEnumerator19"))))